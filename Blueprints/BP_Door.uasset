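; BP_Door is an interactable hinged door that toggles open and closed on Interact.
; A timeline plays or reverses to lerp the door's yaw up to a max angle, signed at BeginPlay by OpenOutside.
; Door collision is disabled on Interact and restored when the timeline finishes.
; Overlapping InteractBox shows the prompt widget and enables custom depth on door and frame.
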(event `self.ReceiveBeginPlay`
  ;[0 0 0] Init
  (set `self.MaxDoorRotateAngle` (* (`KismetMathLibrary.SelectFloat` -1.0 1.0 (`self.OpenOutside`)) (`self.MaxDoorRotateAngle`))))

(event `OpenDoorEvent`
  (bind _door (`self.Door`))
  ;[0 0 0] OpenCloseDoor
  (bind (_direction _value) (`Timeline|Timeline` :!label _label)
    (:`Update`
      (`SceneComponent.K2_SetRelativeRotation` _door (`KismetMathLibrary.MakeRotator` (.roll (`SceneComponent.K2_GetComponentRotation` _door)) (.pitch (`SceneComponent.K2_GetComponentRotation` _door)) (`KismetMathLibrary.Lerp` 0.0 (`self.MaxDoorRotateAngle`) _value)) false false))
    (:`Finished`
      (`PrimitiveComponent.SetCollisionEnabled` (`self.Door`) "QueryAndPhysics"))))

(event `CloseDoorEvent`
  ;[0 0 0] OpenCloseDoor
  (goto _label :!via `Reverse`))

(event `/Game/Hawknest/Blueprints/BPI_Interaction.Interact`
  ;[0 0 0] Interact
  (`PrimitiveComponent.SetCollisionEnabled` (`self.Door`) "NoCollision")
  (bind _output_get (set `self.IsOpened` (not (`self.IsOpened`))))
  (if _output_get
    (`self.OpenDoorEvent`)
    (else
      (`self.CloseDoorEvent`))))

(event `self.InteractBox.OnComponentBeginOverlap`
  (params (OverlappedComponent :type "PrimitiveComponent Object Reference") (OtherActor :type "Actor Object Reference") (OtherComp :type "PrimitiveComponent Object Reference") (OtherBodyIndex :type Integer) (bFromSweep :type Boolean) (SweepResult :type "HitResult Structure (by ref)"))
  (`PrimitiveComponent.SetRenderCustomDepth` (`self.Door`) true)
  (`PrimitiveComponent.SetRenderCustomDepth` (`self.Frame`) true)
  (`SceneComponent.SetHiddenInGame` (`self.Widget`) false false))

(event `self.InteractBox.OnComponentEndOverlap`
  (params (OverlappedComponent :type "PrimitiveComponent Object Reference") (OtherActor :type "Actor Object Reference") (OtherComp :type "PrimitiveComponent Object Reference") (OtherBodyIndex :type Integer))
  (`PrimitiveComponent.SetRenderCustomDepth` (`self.Door`) false)
  (`PrimitiveComponent.SetRenderCustomDepth` (`self.Frame`) false)
  (`SceneComponent.SetHiddenInGame` (`self.Widget`) true false))

(fn `UserConstructionScript`)