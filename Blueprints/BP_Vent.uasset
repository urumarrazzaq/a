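; BP_Vent is a vent prop whose mesh spins continuously around its local roll axis.
; The construction script assigns the configurable Mesh to the SMVent01 component.
; On BeginPlay it scales RotatePerSecons by a random factor to vary the spin speed.
; Tick adds that fixed rotation every frame without delta-time scaling, so the speed depends on frame rate despite the variable's name.
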(event `self.ReceiveBeginPlay`
  (set `self.DeltaRot` (`self.GetRandomDeltaRotation`)))

(event `self.ReceiveTick`
  (params (DeltaSeconds :type "Float (single-precision)"))
  (`SceneComponent.K2_AddLocalRotation` (`self.SM_Vent_01`) (`self.DeltaRot`) false false))

(fn `GetRandomDeltaRotation`
  (returns (ReturnValue :type "Rotator Structure"))
  (return (`KismetMathLibrary.MakeRotator` (* (`self.RotatePerSecons`) (`KismetMathLibrary.RandomFloatInRange` 0.5 1.5)))))

(fn `UserConstructionScript`
  (`StaticMeshComponent.SetStaticMesh` (`self.SM_Vent_01`) (`self.Mesh`)))