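; BP_Air_Coolers is an air cooler Blueprint set up to spin its parts, though the rotation is currently disconnected.
; Tick calls Rota every frame, but that function's body is empty and its three AddLocalRotation nodes never run.
; GetRandomDeltaRotation supplies those unused nodes with a roll-only step from delta seconds and RotatePerSecondL, randomly scaled on each evaluation for an uneven speed.
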(event `self.ReceiveTick`
  (params (DeltaSeconds :type "Float (single-precision)"))
  (`self.Rota`))

(fn `GetRandomDeltaRotation`
  (returns (ReturnValue :type "Rotator Structure"))
  (locals (RotatePerSecond_L :type "Float (double-precision)" :default 1.0))
  (return (`KismetMathLibrary.MakeRotator` (* (`GameplayStatics.GetWorldDeltaSeconds`) (`local.RotatePerSecond_L`) 360.0 (`KismetMathLibrary.RandomFloatInRange` 0.5 1.5)))))

(fn `Rota`)

(fn `UserConstructionScript`)