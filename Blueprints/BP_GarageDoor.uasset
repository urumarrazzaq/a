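; BP_GarageDoor is an interactable garage door that toggles between open and closed.
; Overlapping InteractBox shows the prompt widget and enables custom depth on the door mesh, clearing both on exit.
; Interact plays one opening montage forward or in reverse from the door's current animation position.
; Collision turns off after a short delay when opening and turns back on as soon as closing starts.
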(event `self.InteractBox.OnComponentBeginOverlap`
  (params (OverlappedComponent :type "PrimitiveComponent Object Reference") (OtherActor :type "Actor Object Reference") (OtherComp :type "PrimitiveComponent Object Reference") (OtherBodyIndex :type Integer) (bFromSweep :type Boolean) (SweepResult :type "HitResult Structure (by ref)"))
  (`PrimitiveComponent.SetRenderCustomDepth` (`self.Door`) true)
  (`SceneComponent.SetHiddenInGame` (`self.Widget`) false false))

(event `self.InteractBox.OnComponentEndOverlap`
  (params (OverlappedComponent :type "PrimitiveComponent Object Reference") (OtherActor :type "Actor Object Reference") (OtherComp :type "PrimitiveComponent Object Reference") (OtherBodyIndex :type Integer))
  (`PrimitiveComponent.SetRenderCustomDepth` (`self.Door`) false)
  (`SceneComponent.SetHiddenInGame` (`self.Widget`) true false))

(event `/Game/Hawknest/Blueprints/BPI_Interaction.Interact`
  (bind _door (`self.Door`))
  (bind _returnvalue (`SkeletalMeshComponent.GetPosition` _door))
  (bind _output_get (set `self.IsOpened` (not (`self.IsOpened`))))
  (if _output_get
    (`|PlayMontage` _door "/Game/Hawknest/Meshes/Garage_Door/Animated/Anim_Garage_Door_open_anim_Anim_Montage.Anim_Garage_Door_open_anim_Anim_Montage" 1.0 _returnvalue
      (:`then`
        (`KismetSystemLibrary.Delay` 2.0)
        (`PrimitiveComponent.SetCollisionEnabled` (`self.Door`) "NoCollision")))
    (else
      (`|PlayMontage` _door "/Game/Hawknest/Meshes/Garage_Door/Animated/Anim_Garage_Door_open_anim_Anim_Montage.Anim_Garage_Door_open_anim_Anim_Montage" -1.0 _returnvalue
        (:`then`
          (`PrimitiveComponent.SetCollisionEnabled` (`self.Door`) "QueryAndPhysics"))))))

(fn `UserConstructionScript`)