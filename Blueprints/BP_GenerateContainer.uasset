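; Construction-script Blueprint that generates a 3D grid of copies of one static mesh, apparently stacked containers, sized by per-axis object counts and spacing.
; Nested Z, Y and X loops add a mesh component per cell, each with a dynamic material instance from a randomly picked material.
; Random noise varies yaw and the X/Y spacing before index multiplication, so position jitter grows along the grid, while Z layers stay evenly spaced.
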(fn `UserConstructionScript`
  (bind (_objectlengthxyz_x _objectlengthxyz_y _objectlengthxyz_z) (`KismetMathLibrary.BreakVector` (`self.ObjectLengthXYZ`)))
  (bind (_objectcountxyz_x _objectcountxyz_y _objectcountxyz_z) (break `IntVector` (`self.ObjectCountXYZ`)))
  (bind (_locationnoiseminmax_x _locationnoiseminmax_y) (`KismetMathLibrary.BreakVector2D` (`self.LocationNoiseMinMax`)))
  (bind (_locationnoiseminmax_x_2 _locationnoiseminmax_y_2) (`KismetMathLibrary.BreakVector2D` (`self.LocationNoiseMinMax`)))
  (bind (_rotationnoiseminmax_x _rotationnoiseminmax_y) (`KismetMathLibrary.BreakVector2D` (`self.RotationNoiseMinMax`)))
  (for _index (range _objectcountxyz_z)
    (for _index_2 (range _objectcountxyz_y)
      (for _index_3 (range _objectcountxyz_x)
        (bind _returnvalue (`AddComponent|NODE_AddStaticMeshComponent-0` :`RelativeTransform` (`KismetMathLibrary.MakeTransform` (`KismetMathLibrary.MakeVector` (* _index_3 (`self.GetRandomeNoise` _objectlengthxyz_x _locationnoiseminmax_x _locationnoiseminmax_y)) (* _index_2 (`self.GetRandomeNoise` _objectlengthxyz_y _locationnoiseminmax_x_2 _locationnoiseminmax_y_2)) (* _objectlengthxyz_z _index)) (`KismetMathLibrary.MakeRotator` 0.0 0.0 (`self.GetRandomeNoise` (`self.DefaultRotation`) _rotationnoiseminmax_x _rotationnoiseminmax_y)))))
        (`StaticMeshComponent.SetStaticMesh` _returnvalue (`self.New Mesh`))
        (`PrimitiveComponent.CreateDynamicMaterialInstance` _returnvalue 0 (`KismetArrayLibrary.Array_Random` (`self.Materials`)) "None")))))