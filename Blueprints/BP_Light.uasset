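; BP_Light is a configurable LED floodlight actor that pairs a floodlight mesh with a light component.
; Its construction script feeds the color, intensity and flicker settings into a dynamic instance of the mesh's material, keeping the emissive look in step with the light.
; It also applies color, temperature and intensity to the light and picks a flickering or standard light function material.
; BeginPlay only prints the actor's name when a light function is set.
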(event `self.ReceiveBeginPlay`
  (`/Engine/EditorBlueprintResources/StandardMacros.IsValid` (`LightComponent.LightFunctionMaterial` (`self.Light`))
    (:`Is Valid`
      (`KismetSystemLibrary.PrintString` (`KismetSystemLibrary.GetDisplayName` null)))))

(fn `UserConstructionScript`
  (bind _light_intensity (`self.Light Intensity`))
  (bind _light (`self.Light`))
  (bind _sm_led_floodlight_a (`self.SM_Led_Floodlight_a`))
  (bind _returnvalue (`PrimitiveComponent.CreateDynamicMaterialInstance` _sm_led_floodlight_a 0 (`PrimitiveComponent.GetMaterial` _sm_led_floodlight_a 0) "None"))
  (`MaterialInstanceDynamic.SetScalarParameterValue` _returnvalue "Flicker" (`KismetMathLibrary.Conv_BoolToDouble` (`self.Flicker`)))
  (`MaterialInstanceDynamic.SetVectorParameterValue` _returnvalue "Emissive Color" (`self.Light Color`))
  (`LightComponent.SetLightFunctionMaterial` (`self.Light`) (select `bool` (`self.Flicker`) :`false` "/Game/Hawknest/Materials/MaterialInstance/MI_Light_Function_Inst.MI_Light_Function_Inst" :`true` "/Game/Hawknest/Materials/MaterialInstance/MI_Light_Function_Flicker.MI_Light_Function_Flicker" :!type "MaterialInterface Object Reference"))
  (`MaterialInstanceDynamic.SetScalarParameterValue` _returnvalue "Intensity" _light_intensity)
  (`LightComponent.SetUseTemperature` _light true)
  (`LightComponent.SetTemperature` _light (`self.Light Temperature`))
  (`LightComponent.SetLightColor` _light (`self.Light Color`) true)
  (`LightComponent.SetIntensity` _light _light_intensity))