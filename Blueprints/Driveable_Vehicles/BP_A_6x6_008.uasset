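; BP_A_6x6_008 is a driveable vehicle variant, apparently a 6x6, that specializes a parent vehicle Blueprint.
; It overrides the wheel spawn to pass BP_W_008 as both the front and rear wheel.
; Its light toggle calls the parent, then applies the same visibility to four point lights.
; The event graph is disabled and the construction script only calls the parent, so other behavior is inherited.
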(fn `ToggleLight`
  (params (bNewVisibility :type Boolean))
  (`parent.ToggleLight` bNewVisibility)
  (`SceneComponent.SetVisibility` (`self.PointLight7`) bNewVisibility false)
  (`SceneComponent.SetVisibility` (`self.PointLight6`) bNewVisibility false)
  (`SceneComponent.SetVisibility` (`self.PointLight9`) bNewVisibility false)
  (`SceneComponent.SetVisibility` (`self.PointLight8`) bNewVisibility false))

(fn `UserConstructionScript`
  (`parent.UserConstructionScript`))

(fn `Wheels_Spawn`
  (params (FrontWheel :type "Actor Class Reference") (RearWheel :type "Actor Class Reference"))
  (`parent.Wheels_Spawn` "/Game/Hawknest/Blueprints/Driveable_Vehicles/BP_W_008.BP_W_008_C" "/Game/Hawknest/Blueprints/Driveable_Vehicles/BP_W_008.BP_W_008_C"))