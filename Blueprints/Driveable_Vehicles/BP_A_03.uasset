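; BP_A_03 is a driveable vehicle Blueprint that adds a toggle for two flasher components on top of its parent class.
; Pressing the 1 key runs a FlipFlop that alternately shows and hides Flasher and Flasher1, without propagating to child components.
; BeginPlay, Tick and the construction script only call the parent, and the overlap event is disabled.
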(event `self.ReceiveBeginPlay`
  (`parent.ReceiveBeginPlay`))

(event `Key|One`
  (params (Key :type "Key Structure"))
  (bind _flasher (`self.Flasher`))
  (:`Pressed`
    (`/Engine/EditorBlueprintResources/StandardMacros.FlipFlop`
      (:`A`
        (`SceneComponent.SetVisibility` _flasher true false)
        (`SceneComponent.SetVisibility` (`self.Flasher1`) true false))
      (:`B`
        (`SceneComponent.SetVisibility` _flasher false false)
        (`SceneComponent.SetVisibility` (`self.Flasher1`) false false)))))

(event `self.ReceiveTick`
  (params (DeltaSeconds :type "Float (single-precision)"))
  (`parent.ReceiveTick` DeltaSeconds))

(fn `UserConstructionScript`
  (`parent.UserConstructionScript`))