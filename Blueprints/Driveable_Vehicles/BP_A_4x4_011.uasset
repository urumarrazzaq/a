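; BP_A_4x4_011 is a drivable 4x4 vehicle variant that tows a trailer.
; On BeginPlay it spawns the class chosen by TrailerIndex at the mesh's TrailerSocket, passing BaseTrailerIndex as the trailer type.
; A physics constraint then joins the root bones of the vehicle and trailer meshes.
; It overrides the parent's wheel spawning with its own front and rear 011 wheel classes; AddTrailer is an empty stub.
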(event `self.ReceiveBeginPlay`
  (`parent.ReceiveBeginPlay`)
  (bind _returnvalue (`|SpawnActorFromClass` (`|GetArrayItem` (`self.TrailerClasses`) (`self.TrailerIndex`)) (`SceneComponent.GetSocketTransform` (`self.Mesh`) "TrailerSocket" "RTS_World") "Undefined" "OverrideRootScale" null (`self.BaseTrailerIndex`) null))
  (`/Engine/EditorBlueprintResources/StandardMacros.IsValid` _returnvalue
    (:`Is Valid`
      (bind _output_get (set `self.Trail` _returnvalue))
      (`PhysicsConstraintComponent.SetConstrainedComponents` (`self.PhysicsConstraint`) (`self.Mesh`) "root" (`WheeledVehiclePawn.Mesh` _output_get) "root"))))

(fn `Add Trailer`)

(fn `UserConstructionScript`
  (`parent.UserConstructionScript`))

(fn `Wheels_Spawn`
  (params (FrontWheel :type "Actor Class Reference") (RearWheel :type "Actor Class Reference"))
  (`parent.Wheels_Spawn` "/Game/Hawknest/Blueprints/Driveable_Vehicles/BP_W_011_F.BP_W_011_F_C" "/Game/Hawknest/Blueprints/Driveable_Vehicles/BP_W_011_R.BP_W_011_R_C"))