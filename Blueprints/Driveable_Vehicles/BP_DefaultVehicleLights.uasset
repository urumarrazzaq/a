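; Vehicle Blueprint that handles the headlights and brake lights of a driveable vehicle.
; The Light input toggles the left and right spotlights on and off through a FlipFlop.
; Brake and handbrake inputs share one BrakeLights function, which shows the rear brake, parking and reverse light components on press and hides them on release.
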(event `InputAction|Light`
  (params (Key :type "Key Structure"))
  (bind _left_spot_light (`self.Left Spot Light`))
  (:`Pressed`
    (`/Engine/EditorBlueprintResources/StandardMacros.FlipFlop`
      (:`A`
        (`SceneComponent.SetVisibility` _left_spot_light true false)
        (`SceneComponent.SetVisibility` (`self.Right Spot Light`) true false))
      (:`B`
        (`SceneComponent.SetVisibility` _left_spot_light false false)
        (`SceneComponent.SetVisibility` (`self.Right Spot Light`) false false)))))

(event `EnhancedInput|/Game/Hawknest/Blueprints/Driveable_Vehicles/Input/Actions/IA_Break`
  (params (ActionValue :type "Float (double-precision)") (ElapsedSeconds :type "Float (double-precision)") (TriggeredSeconds :type "Float (double-precision)") (InputAction :type "InputAction Object Reference" :default "/Game/Hawknest/Blueprints/Driveable_Vehicles/Input/Actions/IA_Break.IA_Break"))
  (:`Started`
    (`self.BrakeLights` true :!label _label))
  (:`Completed`
    (`self.BrakeLights` false :!label _label_2)))

(event `EnhancedInput|/Game/Hawknest/Blueprints/Driveable_Vehicles/Input/Actions/IA_Handbrake`
  (params (ActionValue :type Boolean) (ElapsedSeconds :type "Float (double-precision)") (TriggeredSeconds :type "Float (double-precision)") (InputAction :type "InputAction Object Reference" :default "/Game/Hawknest/Blueprints/Driveable_Vehicles/Input/Actions/IA_Handbrake.IA_Handbrake"))
  (:`Started`
    (goto _label))
  (:`Completed`
    (goto _label_2)))

(fn `BrakeLights`
  (params (BrakeLights :type Boolean))
  (`SceneComponent.SetVisibility` (`self.Brake Light Left1`) BrakeLights false)
  (`SceneComponent.SetVisibility` (`self.Parking lights Left1`) BrakeLights false)
  (`SceneComponent.SetVisibility` (`self.Reverse2`) BrakeLights false)
  (`SceneComponent.SetVisibility` (`self.Parking lights Right1`) BrakeLights false)
  (`SceneComponent.SetVisibility` (`self.Brake Light Right1`) BrakeLights false)
  (`SceneComponent.SetVisibility` (`self.Reverse3`) BrakeLights false)
  (`SceneComponent.SetVisibility` (`self.Brake Light Left2`) BrakeLights false))

(fn `UserConstructionScript`
  (`parent.UserConstructionScript`))