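; BP_Base_Wheel is a base vehicle wheel that drives a tire material effect, likely squash, from ground contact.
; Each Tick it line-traces from the Tire bounds center down one sphere radius, ignoring every BP_Base_Truck found that frame.
; The hit's height above that bottom point is clamped, rescaled and written to the tire materials' "Add" scalar parameter, without checking whether the trace hit.
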(event `self.ReceiveTick`
  (params (DeltaSeconds :type "Float (single-precision)"))
  (bind (_origin _boxextent _sphereradius) (`KismetSystemLibrary.GetComponentBounds` (`self.Tire`)))
  (bind _returnvalue (`KismetMathLibrary.MakeVector` (.x _origin) (.y _origin) (- (.z _origin) _sphereradius)))
  (`|ExecutionSequence`
    (:`then_0`
      (bind _outactors (`GameplayStatics.GetAllActorsOfClass` "/Game/Hawknest/Blueprints/Driveable_Vehicles/BP_Base_Truck.BP_Base_Truck_C"))
      (bind _outhit (`KismetSystemLibrary.LineTraceSingle` _origin _returnvalue "TraceTypeQuery1" true _outactors))
      (bind (_returnvalue_x _returnvalue_y _returnvalue_z) (`KismetMathLibrary.BreakVector` (- _returnvalue (`.Location` (`GameplayStatics.BreakHitResult` _outhit)))))
      (`MeshComponent.SetScalarParameterValueOnMaterials` (`self.Tire`) "Add" (* (/ (`KismetMathLibrary.FClamp` (* _returnvalue_z -1.0) 0.0 20.0) 20.0) 100.0)))))

(fn `UserConstructionScript`)